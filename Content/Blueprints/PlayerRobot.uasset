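; Player-controlled robot pawn that handles intro dialogue, death and the escape win condition.
; On possession by a player controller it chains three intro lines through Say.
; Tick watches for negative Health, or for the capsule dropping below a fixed height, which counts as escaping and plays the win line.
; Both endings share a delayed fade to black and reload the Default map; K applies lethal self-damage.
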(event EventBeginPlay)

(event Collision|EventActorBeginOverlap
  (params (OtherActor :type Actor%20Object%20Reference)))

(event EventTick
  (params (DeltaSeconds :type Float%20%28single-precision%29))
  (if (and (< (Variables|Default|GetHealth) 0.0) (not (Variables|Default|GetHasDied)))
    (Variables|Default|SetHasDied true)
    (Utilities|FlowControl|Delay 2.0 :!label _label)
    (bind _returnvalue (UserInterface|CreateWidget "/Game/UI/FadeToBlack.FadeToBlack_C"))
    (UserInterface|Viewport|AddtoViewport _returnvalue 0)
    (Utilities|FlowControl|Delay 2.0)
    (Game|OpenLevel(byName) "/Game/Maps/Default")
    (elif (< (.Z (Math|Vector|BreakVector (Transformation|GetWorldLocation (Variables|Default|GetCapsuleComponent)))) 115.0)
      (if (not (Variables|Default|GetHaveEscaped))
        (Variables|Default|SetHaveEscaped true)
        (Utilities|Say "win" 0.0
          (:Done
            (goto _label)))))))

(event EventPossessed
  (params (NewController :type Controller%20Object%20Reference))
  (Utilities|Casting|CastToPlayerController NewController)
  (Utilities|Say "intro0" 0.0
    (:Done
      (Utilities|Say "intro1" 4.0
        (:Done
          (Utilities|Say "intro2" 8.0))))))

(event Input|KeyboardEvents|K
  (params (Key :type Key%20Structure :default "AnyKey"))
  (:Pressed
    (Game|Damage|ApplyDamage self 5e+03 0 0)))

(fn ConstructionScript
  (|CallParentFunction))