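; BaseRobot is a robot Blueprint that displays its health through a material on its Cube component.
; On BeginPlay it creates a dynamic material instance from the Cube's first material slot and stores it as EyeMaterial.
; Every Tick it writes the ratio of Health to MaxHealth into that material's HealthPct scalar parameter.
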(event EventBeginPlay
  (bind _returnvalue (Rendering|Material|CreateDynamicMaterialInstance (Variables|Default|GetCube) 0 0 :!class /Script/Engine.PrimitiveComponent))
  (Variables|Default|SetEyeMaterial _returnvalue))

(event Collision|EventActorBeginOverlap
  (params (OtherActor :type Actor%20Object%20Reference)))

(event EventTick
  (params (DeltaSeconds :type Float%20%28single-precision%29))
  (Rendering|Material|SetScalarParameterValue (Variables|Default|GetEyeMaterial) "HealthPct" (/ (Variables|Default|GetHealth) (Variables|Default|GetMaxHealth)) :!class /Script/Engine.MaterialInstanceDynamic))

(fn ConstructionScript)